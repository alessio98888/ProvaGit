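; Drivable car Blueprint that maps player axis inputs to vehicle movement and camera control.
; Throttle, brake and steering axes pass straight into the VehicleMovementComponent.
; LookUp and LookRight share one SetRelativeRotation node that adds axis input to the SpringArm's current pitch and yaw, with roll held at zero.
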(event Input|AxisEvents|InputAxisthrottle
  (params (AxisValue :type Float%20%28single-precision%29))
  (Class|ChaosVehicleMovementComponent|SetThrottleInput (Variables|Default|GetVehicleMovementComponent) AxisValue))

(event Input|AxisEvents|InputAxisBrake
  (params (AxisValue :type Float%20%28single-precision%29))
  (Class|ChaosVehicleMovementComponent|SetBrakeInput (Variables|Default|GetVehicleMovementComponent) AxisValue))

(event Input|AxisEvents|InputAxisMoveRight
  (params (AxisValue :type Float%20%28single-precision%29))
  (Class|ChaosVehicleMovementComponent|SetSteeringInput (Variables|Default|GetVehicleMovementComponent) AxisValue))

(event Input|AxisEvents|InputAxisLookUp
  (params (AxisValue :type Float%20%28single-precision%29))
  (bind _springarm (Variables|Default|GetSpringArm))
  (bind _returnvalue (Transformation|GetRelativeTransform _springarm))
  (Transformation|SetRelativeRotation _springarm (Math|Rotator|MakeRotator 0.0 (+ AxisValue (.pitch (.rotation _returnvalue))) (+ (.yaw (.rotation _returnvalue)) (stale Input|AxisEvents|InputAxisLookRight AxisValue))) false false))

(event Input|AxisEvents|InputAxisLookRight
  (params (AxisValue :type Float%20%28single-precision%29))
  (bind _springarm (Variables|Default|GetSpringArm))
  (bind _returnvalue (Transformation|GetRelativeTransform _springarm))
  (Transformation|SetRelativeRotation _springarm (Math|Rotator|MakeRotator 0.0 (+ (stale Input|AxisEvents|InputAxisLookUp AxisValue) (.pitch (.rotation _returnvalue))) (+ (.yaw (.rotation _returnvalue)) AxisValue)) false false))

(fn ConstructionScript)